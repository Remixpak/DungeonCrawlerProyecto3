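; BP_Projectile11 is a projectile actor from the Stylized_Projectiles folder that handles its muzzle, flight and impact effects.
; On BeginPlay it spawns MuzzleFX at the Sphere's location and assigns ProjectileFX to the component named Muzzle.
; Any Hit destroys the actor, and the Destroyed event spawns HitFX at the Sphere, so the impact effect plays however the actor is destroyed.
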(event Collision|EventHit
  (params (MyComp :type Primitive%20Component%20Object%20Reference) (Other :type Actor%20Object%20Reference) (OtherComp :type Primitive%20Component%20Object%20Reference) (bSelfMoved :type Boolean) (HitLocation :type Vector :default "0, 0, 0") (HitNormal :type Vector :default "0, 0, 0") (NormalImpulse :type Vector :default "0, 0, 0") (Hit :type Hit%20Result%20Structure%20%28by%20ref%29))
  (Actor|DestroyActor))

(event EventBeginPlay
  (Niagara|SpawnSystematLocation (Variables|Default|GetMuzzle%20FX) (Transformation|GetWorldLocation (Variables|Default|GetSphere)))
  (Class|NiagaraComponent|SetAsset (Variables|Default|GetMuzzle) (Variables|Default|GetProjectile%20FX) true))

(event EventDestroyed
  (Niagara|SpawnSystematLocation (Variables|Default|GetHit%20FX) (Transformation|GetWorldLocation (Variables|Default|GetSphere))))

(fn ConstructionScript)