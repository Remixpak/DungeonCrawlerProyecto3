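; Dungeon game mode that tracks score, colored key pickups and opened chests, and handles level restart and single-slot save/load.
; Reaching the goal score prints a win message and changes the main character's material.
; Check functions destroy tagged keys already collected and chests in rooms marked opened.
; BP_Save stores player transform, room, coins, key flags, and aura, max health and key inventory read from character components.
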(event Custom|AddScore
  (params (ScoreToAdd :type Integer))
  (bind _output_get (Variables|Default|SetCurrentPoints (+ (Variables|Default|GetCurrentPoints) ScoreToAdd)))
  (Development|PrintString (select (>= _output_get (Variables|Default|GetGoalPoints)) (Utilities|String|Append "Has Ganado con: " (Utilities|String|ToString(Integer) _output_get)) (Utilities|String|ToString(Integer) _output_get)))
  (if (>= _output_get (Variables|Default|GetGoalPoints))
    (bind _asbp_main_character (Utilities|Casting|CastToBP_MainCharacter (Game|GetPlayerCharacter 0)))
    (bind _output_get_2 (Variables|Default|SetAs%20BP%20Main%20Character _asbp_main_character))
    (Default|ChangeColor _output_get_2 "/Game/StarterContent/Props/Materials/M_TableRound.M_TableRound")))

(event Custom|RestartGame
  (bind _returnvalue (Game|GetCurrentLevelName true))
  (Game|OpenLevel(byName) (Utilities|String|StringToName _returnvalue)))

(event EventBeginPlay)

(fn ConstructionScript)

(fn CheckOpenedChest
  (params (RoomName :type String))
  (if (and (Utilities|Map|Contains (Variables|Default|GetOpenedChest) RoomName) (.Value (Utilities|Map|Find (Variables|Default|GetOpenedChest) RoomName)))
    (bind _outactors (Actor|GetAllActorswithTag "Chest"))
    (for _array_element _outactors
      (Actor|DestroyActor _array_element))))

(fn CheckCollectedKeys
  (bind _outactors (Actor|GetAllActorswithTag "Key"))
  (for _array_element _outactors
    (bind _asbp_key_pickup (Utilities|Casting|CastToBP_KeyPickup _array_element))
    (switch Utilities|FlowControl|Switch|SwitchonE_KeyColor (Variables|/Game/GameLogic/GameplaySystems/UnlockDoorsSystem/BP_KeyPickup.BP_KeyPickup_C|GetKeyColor _asbp_key_pickup)
      (:NewEnumerator0
        (if (Variables|Default|GetGotRedKey)
          (Actor|DestroyActor _asbp_key_pickup)))
      (:NewEnumerator1
        (if (Variables|Default|GetGotBlueKey)
          (Actor|DestroyActor _asbp_key_pickup)))
      (:NewEnumerator2
        (if (Variables|Default|GetGotGreenKey)
          (Actor|DestroyActor _asbp_key_pickup))))))

(fn SaveGame
  (bind _returnvalue (Game|Player|GetPlayerPawn 0))
  (bind _returnvalue_2 (SaveGame|CreateSaveGameObject "/Game/GameLogic/BP_Save.BP_Save_C"))
  (Variables|/Game/GameLogic/BP_Save.BP_Save_C|SetPlayerTransform _returnvalue_2 (Transformation|GetActorTransform _returnvalue))
  (Variables|/Game/GameLogic/BP_Save.BP_Save_C|SetLoadedRoom _returnvalue_2 (Variables|Default|GetLoadedRoom))
  (bind _asbp_third_person_character (Utilities|Casting|CastToBP_ThirdPersonCharacter _returnvalue))
  (Variables|/Game/GameLogic/BP_Save.BP_Save_C|SetCurrentAura _returnvalue_2 (Variables|/Elemental_PowerUps_and_Blocks/Source/Components/BP_AuraComponent.BP_AuraComponent_C|GetAuraType (Actor|GetComponentbyClass _asbp_third_person_character "/Elemental_PowerUps_and_Blocks/Source/Components/BP_AuraComponent.BP_AuraComponent_C")))
  (Variables|/Game/GameLogic/BP_Save.BP_Save_C|SetHealth _returnvalue_2 (Variables|/Script/MyProject.HealthSystemComponent|GetMaxHealth (Actor|GetComponentbyClass _asbp_third_person_character "/Game/GameLogic/GameplaySystems/HealthSystem/BPC_HealthSystemComponent.BPC_HealthSystemComponent_C")))
  (Variables|/Game/GameLogic/BP_Save.BP_Save_C|SetKeys _returnvalue_2 (Variables|/Game/GameLogic/GameplaySystems/UnlockDoorsSystem/BP_KeyInventoryComponent.BP_KeyInventoryComponent_C|GetKeys (Actor|GetComponentbyClass _asbp_third_person_character "/Game/GameLogic/GameplaySystems/UnlockDoorsSystem/BP_KeyInventoryComponent.BP_KeyInventoryComponent_C")))
  (Variables|/Game/GameLogic/BP_Save.BP_Save_C|SetGotRedKey _returnvalue_2 (Variables|Default|GetGotRedKey))
  (Variables|/Game/GameLogic/BP_Save.BP_Save_C|SetGotGreenKey _returnvalue_2 (Variables|Default|GetGotGreenKey))
  (Variables|/Game/GameLogic/BP_Save.BP_Save_C|SetGotBlueKey _returnvalue_2 (Variables|Default|GetGotBlueKey))
  (Variables|/Game/GameLogic/BP_Save.BP_Save_C|SetCoins _returnvalue_2 (Variables|Default|GetCurrentPlayerCoins))
  (SaveGame|SaveGametoSlot _returnvalue_2 "1")
  (return))

(fn LoadGame
  (bind _returnvalue (Game|Player|GetPlayerPawn 0))
  (bind _returnvalue_2 (SaveGame|DoesSaveGameExist "1"))
  (if _returnvalue_2
    (bind _returnvalue_3 (SaveGame|LoadGamefromSlot "1"))
    (bind _asbp_save (Utilities|Casting|CastToBP_Save _returnvalue_3))
    (bind _output_get (Variables|Default|SetAs%20BP%20Save _asbp_save))
    (Transformation|SetActorTransform _returnvalue (Variables|/Game/GameLogic/BP_Save.BP_Save_C|GetPlayerTransform _output_get))
    (Variables|Default|SetRoomToLoad (Variables|/Game/GameLogic/BP_Save.BP_Save_C|GetLoadedRoom _output_get))
    (bind _asbp_third_person_character (Utilities|Casting|CastToBP_ThirdPersonCharacter _returnvalue))
    (Default|SetAura (Actor|GetComponentbyClass _asbp_third_person_character "/Elemental_PowerUps_and_Blocks/Source/Components/BP_AuraComponent.BP_AuraComponent_C") (Variables|/Game/GameLogic/BP_Save.BP_Save_C|GetCurrentAura _output_get))
    (Variables|/Script/MyProject.HealthSystemComponent|SetMaxHealth (Actor|GetComponentbyClass _asbp_third_person_character "/Game/GameLogic/GameplaySystems/HealthSystem/BPC_HealthSystemComponent.BPC_HealthSystemComponent_C") (Variables|/Game/GameLogic/BP_Save.BP_Save_C|GetHealth _output_get))
    (for _array_element (Variables|/Game/GameLogic/BP_Save.BP_Save_C|GetKeys _output_get)
      (Default|AddKey (Actor|GetComponentbyClass _asbp_third_person_character "/Game/GameLogic/GameplaySystems/UnlockDoorsSystem/BP_KeyInventoryComponent.BP_KeyInventoryComponent_C") _array_element))
    (Variables|Default|SetGotRedKey (Variables|/Game/GameLogic/BP_Save.BP_Save_C|GetGotRedKey _output_get))
    (Variables|Default|SetGotBlueKey (Variables|/Game/GameLogic/BP_Save.BP_Save_C|GetGotBlueKey _output_get))
    (Variables|Default|SetGotGreenKey (Variables|/Game/GameLogic/BP_Save.BP_Save_C|GetGotGreenKey _output_get))
    (Default|AddCoins _asbp_third_person_character (Variables|/Game/GameLogic/BP_Save.BP_Save_C|GetCoins _output_get))
    (return)
    (else
      (Development|PrintString "No Save file"))))