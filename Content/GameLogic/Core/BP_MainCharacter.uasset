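; BP_MainCharacter is a character Blueprint that gives its mesh a random color when play begins.
; BeginPlay creates a dynamic instance of M_Color, stores it as DynamicMaterial and applies it to the mesh's first material slot.
; The Color parameter comes from a random unit vector scaled by a random float, so negative channels are possible.
; A ChangeColor event takes a material input but has no logic.
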(event Custom|ChangeColor
  (params (Material :type Material%20Interface%20Object%20Reference)))

(event EventBeginPlay
  (bind _returnvalue (Rendering|Material|CreateDynamicMaterialInstance "/Game/Assets/Shaders/M_Color.M_Color" "None" "None" :!class /Script/Engine.KismetMaterialLibrary))
  (Variables|Default|SetDynamicMaterial _returnvalue)
  (Rendering|Material|SetMaterial (Variables|Character|GetMesh) 0 (Variables|Default|GetDynamicMaterial))
  (Rendering|Material|SetVectorParameterValue (Variables|Default|GetDynamicMaterial) "Color" (Math|Conversions|ToLinearColor(Vector) (* (Math|Random|RandomUnitVector) (Math|Random|RandomFloat))) :!class /Script/Engine.MaterialInstanceDynamic))

(event Collision|EventActorBeginOverlap
  (params (OtherActor :type Actor%20Object%20Reference)))

(event EventTick
  (params (DeltaSeconds :type Float%20%28single-precision%29)))

(fn ConstructionScript
  (|CallParentFunction))