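; Health system actor component that reacts to damage on the third-person character and triggers game over when health runs out.
; At BeginPlay it binds to its OnDamageReceived dispatcher, whose handler pushes truncated MaxHealth to the owner's HUD and prints it as current health.
; At zero or below, it shows the HUD game-over screen after a short delay, provided the game mode is BP_GM_Dungeon.
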(event Custom|OnDamageReceived_Event
  (bind _maxhealth (Variables|Default|GetMaxHealth))
  ;[0.15 0.15 0.15 0.5] Damage Logic
  (bind _asbp_third_person_character (Utilities|Casting|CastToBP_ThirdPersonCharacter (Components|GetOwner)))
  (Default|UpdateHealth (Variables|/Game/ThirdPerson/Blueprints/BP_ThirdPersonCharacter.BP_ThirdPersonCharacter_C|GetMy_HUD _asbp_third_person_character) (Math|Float|Truncate _maxhealth))
  (Development|PrintString (Utilities|String|Append (Utilities|String|MakeLiteralString "Vida actual: ") (Utilities|String|ToString(Float) _maxhealth)))
  (if (<= _maxhealth 0.0)
    (Utilities|Casting|CastToBP_GM_Dungeon (Game|GetGameMode))
    (Utilities|FlowControl|Delay 3.0)
    (Default|Activate/DeactivateGameOver (Variables|/Game/ThirdPerson/Blueprints/BP_ThirdPersonCharacter.BP_ThirdPersonCharacter_C|GetMy_HUD _asbp_third_person_character) true)))

(event EventBeginPlay
  ;[0.15 0.15 0.15 0.5] Damage Logic
  (EventDispatchers|AssignOnDamageReceived (delegate Custom|OnDamageReceived_Event)))