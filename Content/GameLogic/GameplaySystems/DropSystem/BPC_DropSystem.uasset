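; BPC_DropSystem is a component that awards coins to the player when its DropCoins event is called.
; A flag limits the award to once, then it adds its Coins value to CurrentPlayerCoins on the BP_GM_Dungeon game mode.
; It prints a Spanish "coins obtained" debug message, which shows the new total rather than the amount just awarded.
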(event Custom|DropCoins
  (if (not (Variables|Default|GetAlreadyDropped?))
    (Variables|Default|SetAlreadyDropped? true)
    (bind _asbp_gm_dungeon (Utilities|Casting|CastToBP_GM_Dungeon (Game|GetGameMode)))
    (bind _output_get (Variables|/Game/GameLogic/Core/BP_GM_Dungeon.BP_GM_Dungeon_C|SetCurrentPlayerCoins _asbp_gm_dungeon (+ (Variables|/Game/GameLogic/Core/BP_GM_Dungeon.BP_GM_Dungeon_C|GetCurrentPlayerCoins _asbp_gm_dungeon) (Variables|Default|GetCoins))))
    (Development|PrintString (Utilities|String|Append (Utilities|String|Append (Utilities|String|MakeLiteralString "¡Has obtenido ") (Utilities|String|ToString(Integer) _output_get)) (Utilities|String|MakeLiteralString " monedas!")) true true "(R=1.000000,G=0.027013,B=0.000000,A=1.000000)")))

(event EventBeginPlay)

(event EventTick
  (params (DeltaSeconds :type Float%20%28single-precision%29)))