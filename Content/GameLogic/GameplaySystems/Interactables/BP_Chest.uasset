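; BP_Chest is a one-time interactable chest that gives coins to the player character.
; On Interact it marks itself opened, adds CoinsToGive to the third-person character and swaps its mesh to a transparent material.
; It then records its Room in the dungeon game mode's OpenedChest map and prints the Room.
; CanInteract returns false once the chest has been opened.
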(event EventBeginPlay)

(event Collision|EventActorBeginOverlap
  (params (OtherActor :type Actor%20Object%20Reference)))

(event EventTick
  (params (DeltaSeconds :type Float%20%28single-precision%29)))

(event EventInteract
  (params (Actor :type Actor%20Object%20Reference))
  (bind _room (Variables|Default|GetRoom))
  ;[0.15 0.15 0.15 0.5] Interaction Logic
  (Variables|Default|SetbOpened true)
  (bind _asbp_third_person_character (Utilities|Casting|CastToBP_ThirdPersonCharacter Actor))
  (Default|AddCoins _asbp_third_person_character (Variables|Default|GetCoinsToGive))
  (Rendering|Material|SetMaterial (Variables|Default|Getcc0_chest) 0 "/Game/Assets/Shaders/M_Transparent.M_Transparent")
  (bind _asbp_gm_dungeon (Utilities|Casting|CastToBP_GM_Dungeon (Game|GetGameMode)))
  (Utilities|Map|Add (Variables|/Game/GameLogic/Core/BP_GM_Dungeon.BP_GM_Dungeon_C|GetOpenedChest _asbp_gm_dungeon) _room true)
  (Development|PrintString _room))

(fn ConstructionScript)

(fn CanInteract
  (params (Actor :type Actor%20Object%20Reference))
  ;[0.15 0.15 0.15 0.5] Cant Interact function
  (if (Variables|Default|GetbOpened)
    (return false)
    (else
      (return true))))