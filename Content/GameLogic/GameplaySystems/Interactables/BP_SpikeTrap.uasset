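; BP_SpikeTrap is an interactable spike trap that damages the player character while armed.
; Interact toggles the Active flag, switching the Box's collision on or off, flipping and repositioning the spike mesh, and printing a Spanish status message.
; When Box begins overlapping a BP_ThirdPersonCharacter while active, it calls that character's ApplyDamage with the damage amount and the trap's location.
; CanInteract always returns true, so any actor can toggle it.
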(event OnComponentBeginOverlap(Box)
  (params (OverlappedComponent :type Primitive%20Component%20Object%20Reference) (OtherActor :type Actor%20Object%20Reference) (OtherComp :type Primitive%20Component%20Object%20Reference) (OtherBodyIndex :type Integer) (bFromSweep :type Boolean) (SweepResult :type Hit%20Result%20Structure%20%28by%20ref%29))
  ;[0.15 0.15 0.15 0.5] Interaction Logic
  (if (Variables|Default|GetbActive)
    (bind _asbp_third_person_character (Utilities|Casting|CastToBP_ThirdPersonCharacter OtherActor))
    (Default|ApplyDamage _asbp_third_person_character (Variables|Default|GetDamageAmount) (Transformation|GetActorLocation))))

(event EventBeginPlay)

(event Collision|EventActorBeginOverlap
  (params (OtherActor :type Actor%20Object%20Reference)))

(event EventTick
  (params (DeltaSeconds :type Float%20%28single-precision%29)))

(event EventInteract
  (params (Actor :type Actor%20Object%20Reference))
  (bind _spike_trap_01 (Variables|Default|Getspike_trap_01))
  (bind _box (Variables|Default|GetBox))
  ;[0.15 0.15 0.15 0.5] Interaction Logic
  (if (Variables|Default|GetbActive)
    (Collision|SetCollisionEnabled _box "NoCollision")
    (Variables|Default|SetbActive false)
    (Development|PrintString "Se desactivo la trampa" true true "(R=0.000000,G=1.000000,B=0.138169,A=1.000000)")
    (Transformation|SetRelativeRotation _spike_trap_01 "0.000000,0.000000,180.000000" false false)
    (Transformation|SetRelativeLocation _spike_trap_01 "0.000000,0.000000,-26.000000" false false)
    (else
      (Collision|SetCollisionEnabled _box "QueryAndPhysics")
      (Variables|Default|SetbActive true)
      (Development|PrintString "Se activo la trampa" true true "(R=0.000000,G=1.000000,B=0.080409,A=1.000000)")
      (Transformation|SetRelativeRotation _spike_trap_01 "0, 0, 0" false false)
      (Transformation|SetRelativeLocation _spike_trap_01 "0.000000,0.000000,-30.000000" false false))))

(fn ConstructionScript)

(fn CanInteract
  (params (Actor :type Actor%20Object%20Reference))
  (return true))