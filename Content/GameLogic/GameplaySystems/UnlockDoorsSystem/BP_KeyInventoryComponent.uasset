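; BP_KeyInventoryComponent is an inventory component in the door-unlocking system that records which colored keys its owner has obtained.
; AddKey stores a key color in the Keys array only if it is absent, then prints a Spanish pickup message with the color name.
; HasKey reports whether a given color is held, and the component runs no BeginPlay or Tick logic.
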(event EventBeginPlay)

(event EventTick
  (params (DeltaSeconds :type Float%20%28single-precision%29)))

(fn AddKey
  (params (KeyColor :type E_KeyColor%20Enum :default "NewEnumerator0"))
  ;[0.15 0.15 0.15 0.5] Add Key function
  (if (not (Utilities|Array|ContainsItem (Variables|Default|GetKeys) KeyColor))
    (Utilities|Array|AddUnique (Variables|Default|GetKeys) KeyColor)
    (Development|PrintString (Utilities|String|Append (Utilities|String|MakeLiteralString "Has obtenido la llave: ") (Utilities|String|EnumtoString KeyColor)))
    (return)))

(fn HasKey
  (params (KeyColor :type E_KeyColor%20Enum :default "NewEnumerator0"))
  ;[0.15 0.15 0.15 0.5] Has Key function
  (return (Utilities|Array|ContainsItem (Variables|Default|GetKeys) KeyColor)))