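; BP_KeyPickup is a colored key pickup for the dungeon's door-unlocking system.
; On BeginPlay it creates a dynamic material on the key mesh and tints it red, blue or green from KeyColor.
; On overlap with an actor that has a BP_KeyInventoryComponent, it adds the key, sets the matching flag on BP_GM_Dungeon and destroys itself.
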(event EventBeginPlay
  (bind _asbp_gm_dungeon (Utilities|Casting|CastToBP_GM_Dungeon (Game|GetGameMode)))
  ;[0.15 0.15 0.15 0.5] Change Dynamic material
  (Variables|Default|SetAs%20BP%20GM%20Dungeon _asbp_gm_dungeon)
  (bind _returnvalue (Rendering|Material|CreateDynamicMaterialInstance (Variables|Default|GetKey) 0 "/Game/Assets/Shaders/M_Dynamic.M_Dynamic" "None" :!class /Script/Engine.PrimitiveComponent))
  (Rendering|Material|SetMaterial (Variables|Default|GetKey) 0 _returnvalue)
  (Variables|Default|SetKeyMaterial _returnvalue)
  (switch Utilities|FlowControl|Switch|SwitchonE_KeyColor (Variables|Default|GetKeyColor)
    (:NewEnumerator0
      (Rendering|Material|SetVectorParameterValue (Variables|Default|GetKeyMaterial) "BaseColor" "(R=1.000000,G=0.039766,B=0.000000,A=1.000000)" :!class /Script/Engine.MaterialInstanceDynamic))
    (:NewEnumerator1
      (Rendering|Material|SetVectorParameterValue (Variables|Default|GetKeyMaterial) "BaseColor" "(R=0.000000,G=0.046939,B=1.000000,A=1.000000)" :!class /Script/Engine.MaterialInstanceDynamic))
    (:NewEnumerator2
      (Rendering|Material|SetVectorParameterValue (Variables|Default|GetKeyMaterial) "BaseColor" "(R=0.000000,G=1.000000,B=0.090115,A=1.000000)" :!class /Script/Engine.MaterialInstanceDynamic))))

(event Collision|EventActorBeginOverlap
  (params (OtherActor :type Actor%20Object%20Reference))
  (bind _returnvalue (Actor|GetComponentbyClass OtherActor "/Game/GameLogic/GameplaySystems/UnlockDoorsSystem/BP_KeyInventoryComponent.BP_KeyInventoryComponent_C"))
  ;[0.15 0.15 0.15 0.5] Pick Up Behavior
  (if (Utilities|IsValid _returnvalue)
    (Default|AddKey _returnvalue (Variables|Default|GetKeyColor))
    (switch Utilities|FlowControl|Switch|SwitchonE_KeyColor (Variables|Default|GetKeyColor)
      (:NewEnumerator0
        (Variables|/Game/GameLogic/Core/BP_GM_Dungeon.BP_GM_Dungeon_C|SetGotRedKey (Variables|Default|GetAs%20BP%20GM%20Dungeon) true))
      (:NewEnumerator1
        (Variables|/Game/GameLogic/Core/BP_GM_Dungeon.BP_GM_Dungeon_C|SetGotBlueKey (Variables|Default|GetAs%20BP%20GM%20Dungeon) true))
      (:NewEnumerator2
        (Variables|/Game/GameLogic/Core/BP_GM_Dungeon.BP_GM_Dungeon_C|SetGotGreenKey (Variables|Default|GetAs%20BP%20GM%20Dungeon) true)))
    (Actor|DestroyActor)))

(event EventTick
  (params (DeltaSeconds :type Float%20%28single-precision%29)))

(fn ConstructionScript)