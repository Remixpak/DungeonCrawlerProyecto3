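; BP_ShootEnemy is an AI enemy that senses pawns and fires bullets.
; Each tick its capsule spins at RotationSpeed while CanRotate is set, otherwise it snaps to face the player if SeingPlayer is set.
; PawnSensing writes any seen pawn to the AI controller's targetPlayer blackboard key.
; Shoot spawns BP_Bullet at the Muzzle transform; neither its caller nor the code setting the two flags is in this Blueprint.
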(event OnSeePawn(PawnSensing)
  (params (Pawn :type Pawn%20Object%20Reference))
  (bind _asai_controller (Utilities|Casting|CastToAI_Controller (Pawn|GetController)))
  (Utilities|IsValid (AI|GetBlackboard _asai_controller)
    (:Is%20Valid
      (AI|Components|Blackboard|SetValueasObject (AI|GetBlackboard _asai_controller) (Utilities|Name|MakeLiteralName "targetPlayer") Pawn))))

(event EventBeginPlay)

(event EventTick
  (params (DeltaSeconds :type Float%20%28single-precision%29))
  (if (Variables|Default|GetCanRotate)
    (Transformation|AddLocalRotation (Variables|Collision|GetCapsuleComponent) (Math|Rotator|MakeRotator 0.0 0.0 (* (Variables|Default|GetRotationSpeed) (Utilities|Time|GetWorldDeltaSeconds))) false false)
    (elif (Variables|Default|GetseingPlayer)
      (Transformation|SetRelativeRotation (Variables|Collision|GetCapsuleComponent) (Math|Rotator|FindLookatRotation (Transformation|GetActorLocation) (Transformation|GetActorLocation (Game|GetPlayerCharacter 0))) false false))))

(fn ConstructionScript)

(fn Shoot
  (bind _muzzle (Variables|Default|GetMuzzle))
  (Game|SpawnActorfromClass "/Game/GameLogic/BP_Bullet.BP_Bullet_C" (Math|Transform|MakeTransform (Transformation|GetWorldLocation _muzzle) (Transformation|GetWorldRotation _muzzle)) "Undefined" "MultiplyWithRoot" 0 0))